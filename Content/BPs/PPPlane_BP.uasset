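; Moving plane actor that tags the static meshes it passes through with custom depth stencil values, the kind a post-process material can read.
; On BeginPlay a timeline lerps it between two fixed world points along X.
; Each Tick it sets overlapping StaticMeshActors to stencil 1.
; It compares against the previous frame's overlap list to set those it has left to stencil 2.
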(event `self.ReceiveBeginPlay`
  (bind (_direction _alpha) (`Timeline|MovementTM` :!via `PlayFromStart`)
    (:`Update`
      (`self.K2_SetActorLocation` (`KismetMathLibrary.VLerp` (600.0 2270.0 30.0) (-600.0 2270.0 30.0) _alpha)))))

(event `self.ReceiveTick`
  (params (DeltaSeconds :type "Float (single-precision)"))
  (bind _nextoverlapping_actors (`self.NextOverlapping Actors`))
  (bind _output_get (set `self.NextOverlapping Actors` (`self.GetOverlappingActors` "/Script/Engine.StaticMeshActor")))
  (for _array_element (`self.PrevOverlapping Actors`)
    (if (not (`KismetArrayLibrary.Array_Contains` _output_get _array_element))
      (`PrimitiveComponent.SetCustomDepthStencilValue` (`StaticMeshActor.StaticMeshComponent` (cast `StaticMeshActor` _array_element :!pure true)) 2)))
  (for _array_element_2 _nextoverlapping_actors
    (`PrimitiveComponent.SetCustomDepthStencilValue` (`StaticMeshActor.StaticMeshComponent` (cast `StaticMeshActor` _array_element_2 :!pure true)) 1))
  (set `self.PrevOverlapping Actors` _nextoverlapping_actors))

(fn `UserConstructionScript`)