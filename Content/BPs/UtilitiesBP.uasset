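; UtilitiesBP is a set of shared Blueprint helpers for reaching core game objects and printing debug text.
; GetPlayer, GetHUD and GetState fetch the player 0 pawn, the HUD of player controller 0 and the game state, each cast to its custom class.
; Each getter returns a value only on a successful cast.
; 2String Print joins two strings with a colon and prints the result.
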(fn `2String Print`
  (params (`1` :type String) (`2` :type String))
  (`KismetSystemLibrary.PrintString` null (`KismetStringLibrary.Concat_StrStr` `1` ": " `2` " ")))

(fn `GetHUD`
  (returns (HUD :type "/Game/BPs/Player/CustomHUD Object Reference"))
  (bind (_ascustom_hud _bsuccess) (cast `/Game/BPs/Player/CustomHUD` (`PlayerController.GetHUD` (`GameplayStatics.GetPlayerController` null)) :!pure true))
  (return (select `bool` _bsuccess :`true` _ascustom_hud)))

(fn `GetPlayer`
  (returns (`Player Pawn` :type "/Game/BPs/Player/CustomPlayerPawn Object Reference"))
  (bind (_ascustom_player_pawn _bsuccess) (cast `/Game/BPs/Player/CustomPlayerPawn` (`GameplayStatics.GetPlayerPawn` null) :!pure true))
  (return (select `bool` _bsuccess :`true` _ascustom_player_pawn)))

(fn `GetState`
  (returns (State :type "/Game/BPs/Player/CustomGameState Object Reference"))
  (bind (_ascustom_game_state _bsuccess) (cast `/Game/BPs/Player/CustomGameState` (`GameplayStatics.GetGameState` null) :!pure true))
  (return (select `bool` _bsuccess :`true` _ascustom_game_state)))